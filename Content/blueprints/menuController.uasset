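; Menu controller that lets a player drive the menu HUD with Kinect body gestures.
; Each tick it converts skeleton joints to centimetres and, when the first joint is inside a floor range, classifies clap, left or right posture.
; Postures open map selection, select a map, start, go back or quit, followed by a tick-counted cooldown.
; Gameplay posture, jump-state, pause and game-over functions are also defined but not called here.
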(event `self.ReceiveBeginPlay`
  ;[1 1 1] 初始化kinect
  (set `self.switch level` false)
  (bind _returnvalue (`KinectManager.GetSensor` (`KinectBPFunctionLibrary.KinectManager`)))
  (bind _output_get (set `self.has kinect` (> (`KismetArrayLibrary.Array_Length` _returnvalue) 0)))
  (if _output_get
    (bind _output_get_2 (set `self.kinect` (`|GetArrayItem` _returnvalue)))
    (`KinectSensor.InitializeSensor` _output_get_2 null)
    ;[1 1 1] 获取hud
    (bind _asmenu_hud (cast `/Game/ui/menuHUD` (`self.GetHUD` (`GameplayStatics.GetPlayerController` 0))))
    (set `self.menu HUD` _asmenu_hud)
    (`self.InitRangeForKinect`)
    (set `self.is main menu` true)
    (set `self.player posture` "NewEnumerator1")
    (set `self.moving` false)
    (else
      (`KismetSystemLibrary.PrintString` "You don't have connected kinect"))))

(event `self.ReceiveTick`
  (params (DeltaSeconds :type "Float (single-precision)"))
  (bind _kinect (`self.kinect`))
  (bind (_a_x _a_y) (`KismetMathLibrary.BreakVector` (`self.A`)))
  (bind (_d_x _d_y) (`KismetMathLibrary.BreakVector` (`self.D`)))
  (bind _player_skeleton_positions (`self.player skeleton positions`))
  (bind _output_jointposition (break `SkelStruct` (`|GetArrayItem` (`KinectSensor.FSkeletons` _kinect))))
  ;[1 1 1] 获取骨骼位置
  (if (`self.has kinect`)
    (`KinectSensor.UpdateSkeleton` _kinect)
    ;[1 1 1] 将骨骼坐标单位转换成cm
    (for (_array_element _array_index) _output_jointposition
      (bind _returnvalue (* _array_element 100.0))
      (`KismetArrayLibrary.Array_Set` _player_skeleton_positions _array_index _returnvalue)
      (if (== _array_index 0)
        (bind _x (.x _returnvalue))
        (bind _y (.y _returnvalue))
        ;[1 1 1] 判断玩家是否在kinect识别区域内
        (set `self.in kinect range` (and (>= _x _a_x) (<= _x _d_x) (<= _y _d_y) (>= _y _a_y)))))
    (`self.DetectPostureAndSendMessage` _player_skeleton_positions)))

(event `self.ReceiveEndPlay`
  (params (EndPlayReason :type "EEndPlayReason Enum" :default "Destroyed"))
  ;[1 1 1] 关闭kinect
  (if (`self.has kinect`)
    (`KinectSensor.CloseKinect` (`self.kinect`))))

(fn `ChangeState`
  (params (`target state` :type "/Game/DataStructure/PLAYER_STATE Enum" :default "NewEnumerator0"))
  (bind _player_state (`self.player state`))
  (bind _player_character (`self.player character`))
  (switch `/Game/DataStructure/PLAYER_STATE` `target state`
    (:`NewEnumerator0`
      (`RedCharacter.cancelJump` _player_character))
    (:`NewEnumerator2`
      (if (`|EnumEquality` _player_state "NewEnumerator0")
        (`RedCharacter.ReadyJump` _player_character)
        (elif (`|EnumEquality` _player_state "NewEnumerator1")
          (`RedCharacter.ResumeJump` _player_character))))
    (:`NewEnumerator1`
      (`RedCharacter.pauseJump` _player_character))
    (:`NewEnumerator3`
      (`RedCharacter.StartJump` _player_character)))
  (set `self.player state` `target state`))

(fn `Delay`
  (bind _tick (`self.tick`))
  (if (< (`self.t1`) _tick)
    (set `self.moving` false)
    (else
      (set `self.tick` (+ 1.0 _tick)))))

(fn `DetectPostureAndSendMessage`
  (params (`player skeleton position` :type "Array of Vector Structure"))
  (bind _menu_hud (`self.menu HUD`))
  (if (`self.in kinect range`)
    (if (`self.moving`)
      (`self.Delay`)
      (else
        (`self.DetectPostureWhenInMenu` `player skeleton position`)
        (if (`self.is main menu`)
          ;[1 1 1] main menu
          (switch `/Game/DataStructure/posture` (`self.player posture`)
            (:`NewEnumerator3`
              (`/Game/ui/menuHUD.CreateSelectMapMenu` (`self.menu HUD`))
              (set `self.is main menu` false))
            (:`NewEnumerator7`
              (`KismetSystemLibrary.QuitGame` null "Quit")))
          (else
            (switch `/Game/DataStructure/posture` (`self.player posture`)
              (:`NewEnumerator3`
                (`/Game/ui/menuHUD.StartGame` _menu_hud))
              (:`NewEnumerator7`
                (`/Game/ui/menuHUD.BackToMainMenu` _menu_hud)
                (set `self.is main menu` true))
              (:`NewEnumerator8`
                (`/Game/ui/menuHUD.SelectMap` _menu_hud)))))
        (set `self.moving` true)
        (set `self.tick` 0.0)))))

(fn `DetectPostureWhenInMenu`
  (params (`player skeleton position` :type "Array of Vector Structure"))
  (bind _output (`|GetArrayItem` `player skeleton position` (`KismetMathLibrary.Conv_ByteToInt` (enumliteral `/Game/DataStructure/SKELETON_POSITION_INDEX` "NewEnumerator1"))))
  (bind _output_2 (`|GetArrayItem` `player skeleton position` (`KismetMathLibrary.Conv_ByteToInt` (enumliteral `/Game/DataStructure/SKELETON_POSITION_INDEX` "NewEnumerator12"))))
  (bind _output_3 (`|GetArrayItem` `player skeleton position` (`KismetMathLibrary.Conv_ByteToInt` (enumliteral `/Game/DataStructure/SKELETON_POSITION_INDEX` "NewEnumerator8"))))
  (if (`self.clap` _output_3 _output_2)
    (set `self.player posture` "NewEnumerator3")
    (elif (`self.left` _output _output_3)
      (set `self.player posture` "NewEnumerator7")
      (elif (`self.right` _output _output_2)
        (set `self.player posture` "NewEnumerator8")
        (else
          (set `self.player posture` "NewEnumerator1")))))
  (return))

(fn `DetectPostureWhileGaming`
  (params (`player skeleton position` :type "Array of Vector Structure"))
  (bind _output (`|GetArrayItem` `player skeleton position` (`KismetMathLibrary.Conv_ByteToInt` (enumliteral `/Game/DataStructure/SKELETON_POSITION_INDEX` "NewEnumerator1"))))
  (if (`self.outside`)
    (set `self.player posture` "NewEnumerator6")
    (elif (`self.raise right hand` (`|GetArrayItem` `player skeleton position` (`KismetMathLibrary.Conv_ByteToInt` (enumliteral `/Game/DataStructure/SKELETON_POSITION_INDEX` "NewEnumerator12"))) (`|GetArrayItem` `player skeleton position` (`KismetMathLibrary.Conv_ByteToInt` (enumliteral `/Game/DataStructure/SKELETON_POSITION_INDEX` "NewEnumerator8"))) (`|GetArrayItem` `player skeleton position` (`KismetMathLibrary.Conv_ByteToInt` (enumliteral `/Game/DataStructure/SKELETON_POSITION_INDEX` "NewEnumerator4"))))
      (set `self.player posture` "NewEnumerator4")
      (elif (`self.squat` _output)
        (set `self.player posture` "NewEnumerator0")
        (elif (`self.jump` _output)
          (set `self.player posture` "NewEnumerator2")
          (else
            (set `self.player posture` "NewEnumerator1"))))))
  (return))

(fn `Gameover`
  (bind _returnvalue (`GameplayStatics.GetPlayerController` 0))
  (set `self.game state` "NewEnumerator6")
  (bind _returnvalue_2 (`|CreateWidget` "/Game/ui/End.End_C"))
  (bind _output_get (set `self.end menu reference` _returnvalue_2))
  (`UserWidget.AddToViewport` _output_get 0)
  (`WidgetBlueprintLibrary.SetInputMode_GameAndUIEx` _returnvalue)
  (`GameplayStatics.SetGamePaused` true)
  (set `PlayerController.bShowMouseCursor` true _returnvalue))

(fn `InitRangeForKinect`
  (locals (MinZ :type "Float (double-precision)" :default 200.0) (MaxZ :type "Float (double-precision)" :default 300.0))
  (bind _minz (`local.MinZ`))
  (bind _maxz (`local.MaxZ`))
  (bind _returnvalue (/ _minz -2.5))
  (bind _returnvalue_2 (/ _minz 2.5))
  (set `local.MinZ` 200.0)
  (set `local.MaxZ` 300.0)
  (set `self.A` (`KismetMathLibrary.MakeVector` _minz _returnvalue))
  (set `self.B` (`KismetMathLibrary.MakeVector` _minz _returnvalue_2))
  (set `self.C` (`KismetMathLibrary.MakeVector` _maxz _returnvalue))
  (set `self.D` (`KismetMathLibrary.MakeVector` _maxz _returnvalue_2)))

(fn `PauseGame`
  (bind _returnvalue (`GameplayStatics.GetPlayerController` 0))
  (bind _pause_menu_reference (`self.pause menu reference`))
  ;[1 1 1] PauseMenu
  (`/Engine/EditorBlueprintResources/StandardMacros.IsValid` _pause_menu_reference
    (:`Is Valid`
      _)
    (:`Is Not Valid`
      (bind _returnvalue_2 (`|CreateWidget` "/Game/ui/PauseMenu.PauseMenu_C"))
      (set `self.pause menu reference` _returnvalue_2)))
  (`WidgetBlueprintLibrary.SetInputMode_UIOnlyEx` _returnvalue _pause_menu_reference)
  (`UserWidget.AddToViewport` _pause_menu_reference 0)
  (set `PlayerController.bShowMouseCursor` true _returnvalue))

(fn `ResumeTo`
  (params (`player state` :type "/Game/DataStructure/PLAYER_STATE Enum" :default "NewEnumerator0"))
  (bind _player_character (`self.player character`))
  (bind _returnvalue (`|EnumEquality` (`self.pause player state`) "NewEnumerator2"))
  (if (`|EnumEquality` `player state` "NewEnumerator2")
    (if _returnvalue
      (`RedCharacter.ResumeJump` _player_character)
      (else
        (`RedCharacter.ReadyJump` _player_character)))
    (elif _returnvalue
      (`RedCharacter.cancelJump` _player_character)))
  (set `self.player state` `player state`)
  (`Widget.RemoveFromParent` (`self.pause menu reference`)))

(fn `UserConstructionScript`)