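; Kinect motion controller that turns the player's body postures into jump commands for RedCharacterBP.
; Each tick it copies the skeleton in centimetres to kinectHUD, checks the play range and classifies posture by joint thresholds.
; A state machine maps squat to charge and jump to launch, with a tick-counted transit window between charging and cancelling.
; While standing or charging, raising the right hand or leaving range pauses; an in-range clap resumes.
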(event `self.ReceiveBeginPlay`
  ;[1 1 1] 初始化kinect
  (bind _returnvalue (`KinectManager.GetSensor` (`KinectBPFunctionLibrary.KinectManager`)))
  (bind _output_get (set `self.kinect` (`|GetArrayItem` _returnvalue)))
  (`KinectSensor.InitializeSensor` _output_get null)
  ;[1 1 1] 获取hud
  (bind _askinect_hud (cast `/Game/ui/kinectHUD` (`self.GetHUD` (`GameplayStatics.GetPlayerController` 0))))
  (set `self.kinect HUD` _askinect_hud)
  ;[1 1 1] 获取角色
  (bind _asred_character_bp (cast `/Game/Red/RedCharacterBP` (`GameplayStatics.GetPlayerCharacter` 0)))
  (set `self.player character` _asred_character_bp)
  (`self.InitRangeForKinect`)
  (set `self.game state` "NewEnumerator0")
  (set `self.player state` "NewEnumerator0"))

(event `self.ReceiveTick`
  (params (DeltaSeconds :type "Float (single-precision)"))
  (bind _kinect (`self.kinect`))
  (bind (_a_x _a_y) (`KismetMathLibrary.BreakVector` (`self.A`)))
  (bind (_d_x _d_y) (`KismetMathLibrary.BreakVector` (`self.D`)))
  (bind _playerskeletonpositions (`/Game/ui/kinectHUD.PlayerSkeletonPositions` (`self.kinect HUD`)))
  (bind _output_jointposition (break `SkelStruct` (`|GetArrayItem` (`KinectSensor.FSkeletons` _kinect))))
  ;[1 1 1] 获取骨骼位置
  (`KinectSensor.UpdateSkeleton` _kinect)
  ;[1 1 1] 将骨骼坐标单位转换成cm，传给hud绘制
  (for (_array_element _array_index) _output_jointposition
    (bind _returnvalue (* _array_element 100.0))
    (`KismetArrayLibrary.Array_Set` _playerskeletonpositions _array_index _returnvalue)
    (if (== _array_index 0)
      (bind _x (.x _returnvalue))
      (bind _y (.y _returnvalue))
      ;[1 1 1] 判断玩家是否在kinect识别区域内
      (bind _output_get (set `/Game/ui/kinectHUD.in kinect range` (and (>= _x _a_x) (<= _x _d_x) (<= _y _d_y) (>= _y _a_y)) (`self.kinect HUD`)))
      (set `self.in kinect range` _output_get)))
  (`self.DetectPostureAndSendMessage` _playerskeletonpositions))

(event `self.ReceiveEndPlay`
  (params (EndPlayReason :type "EEndPlayReason Enum" :default "Destroyed"))
  ;[1 1 1] 关闭kinect
  (`KinectSensor.CloseKinect` (`self.kinect`)))

(fn `ChangeState`
  (params (`target state` :type "/Game/DataStructure/PLAYER_STATE Enum" :default "NewEnumerator0"))
  (bind _player_state (`self.player state`))
  (bind _player_character (`self.player character`))
  (switch `/Game/DataStructure/PLAYER_STATE` `target state`
    (:`NewEnumerator0`
      (`RedCharacter.cancelJump` _player_character))
    (:`NewEnumerator2`
      (if (`|EnumEquality` _player_state "NewEnumerator0")
        (`RedCharacter.ReadyJump` _player_character)
        (elif (`|EnumEquality` _player_state "NewEnumerator1")
          (`RedCharacter.ResumeJump` _player_character))))
    (:`NewEnumerator1`
      (`RedCharacter.pauseJump` _player_character))
    (:`NewEnumerator3`
      (`RedCharacter.StartJump` _player_character)))
  (set `self.player state` `target state`))

(fn `DetectPostureAndSendMessage`
  (params (`player skeleton position` :type "Array of Vector Structure"))
  (bind _player_posture (`self.player posture`))
  (bind _tick (`self.tick`))
  (switch `/Game/DataStructure/GAME_STATE` (`self.game state`)
    (:`NewEnumerator0`
      (`self.DetectPostureWhileGaming` `player skeleton position`)
      (switch `/Game/DataStructure/PLAYER_STATE` (`self.player state`)
        (:`NewEnumerator0`
          (switch `/Game/DataStructure/posture` _player_posture
            (:`NewEnumerator0`
              (`self.ChangeState` "NewEnumerator2"))
            (:`NewEnumerator2`
              (`self.ChangeState` "NewEnumerator3"))
            (:`NewEnumerator4`
              ;[1 1 1] 暂停游戏
              (set `self.game state` "NewEnumerator1" :!label _label)
              (set `self.pause player state` (`self.player state`)))
            (:`NewEnumerator6`
              (goto _label))))
        (:`NewEnumerator2`
          (switch `/Game/DataStructure/posture` _player_posture
            (:`NewEnumerator1`
              (set `self.tick` 0.0)
              (`self.ChangeState` "NewEnumerator1"))
            (:`NewEnumerator4`
              (goto _label))
            (:`NewEnumerator6`
              (goto _label))))
        (:`NewEnumerator1`
          ;[1 1 1] Transiting
          (switch `/Game/DataStructure/posture` _player_posture
            (:`NewEnumerator0`
              (`self.ChangeState` "NewEnumerator2"))
            (:`NewEnumerator1`
              (if (`self.transit` _tick)
                (bind _output_get (set `self.tick` (+ 1.0 _tick)))
                (`KismetSystemLibrary.PrintString` (`KismetStringLibrary.Conv_DoubleToString` _output_get))
                (else
                  (`self.ChangeState` "NewEnumerator0"))))
            (:`NewEnumerator2`
              (`self.ChangeState` "NewEnumerator3"))))
        (:`NewEnumerator3`
          (switch `/Game/DataStructure/posture` _player_posture
            (:`NewEnumerator1`
              (`self.ChangeState` "NewEnumerator0"))))))
    (:`NewEnumerator1`
      ;[1 1 1] 暂停状态下判断是否有拍手动作
      (if (and (not (`self.outside`)) (`self.clap` (`|GetArrayItem` `player skeleton position` (`KismetMathLibrary.Conv_ByteToInt` (enumliteral `/Game/DataStructure/SKELETON_POSITION_INDEX` "NewEnumerator12"))) (`|GetArrayItem` `player skeleton position` (`KismetMathLibrary.Conv_ByteToInt` (enumliteral `/Game/DataStructure/SKELETON_POSITION_INDEX` "NewEnumerator8")))))
        (set `self.game state` "NewEnumerator0")
        ;[1 1 1] 判断继续游戏时玩家的的状态
        (if (`self.squat` (`|GetArrayItem` `player skeleton position` (`KismetMathLibrary.Conv_ByteToInt` (enumliteral `/Game/DataStructure/SKELETON_POSITION_INDEX` "NewEnumerator1"))))
          (`self.ResumeTo` "NewEnumerator2")
          (else
            (`self.ResumeTo` "NewEnumerator0")))))))

(fn `DetectPostureWhileGaming`
  (params (`player skeleton position` :type "Array of Vector Structure"))
  (bind _output (`|GetArrayItem` `player skeleton position` (`KismetMathLibrary.Conv_ByteToInt` (enumliteral `/Game/DataStructure/SKELETON_POSITION_INDEX` "NewEnumerator1"))))
  (if (`self.outside`)
    (set `self.player posture` "NewEnumerator6")
    (elif (`self.raise right hand` (`|GetArrayItem` `player skeleton position` (`KismetMathLibrary.Conv_ByteToInt` (enumliteral `/Game/DataStructure/SKELETON_POSITION_INDEX` "NewEnumerator12"))) (`|GetArrayItem` `player skeleton position` (`KismetMathLibrary.Conv_ByteToInt` (enumliteral `/Game/DataStructure/SKELETON_POSITION_INDEX` "NewEnumerator8"))) (`|GetArrayItem` `player skeleton position` (`KismetMathLibrary.Conv_ByteToInt` (enumliteral `/Game/DataStructure/SKELETON_POSITION_INDEX` "NewEnumerator4"))))
      (set `self.player posture` "NewEnumerator4")
      (elif (`self.squat` _output)
        (set `self.player posture` "NewEnumerator0")
        (elif (`self.jump` _output)
          (set `self.player posture` "NewEnumerator2")
          (else
            (set `self.player posture` "NewEnumerator1"))))))
  (return))

(fn `InitRangeForKinect`
  (locals (MinZ :type "Float (double-precision)" :default 200.0) (MaxZ :type "Float (double-precision)" :default 300.0))
  (bind _minz (`local.MinZ`))
  (bind _maxz (`local.MaxZ`))
  (bind _returnvalue (/ _minz -2.5))
  (bind _returnvalue_2 (/ _minz 2.5))
  (set `local.MinZ` 200.0)
  (set `local.MaxZ` 300.0)
  (set `self.A` (`KismetMathLibrary.MakeVector` _minz _returnvalue))
  (set `self.B` (`KismetMathLibrary.MakeVector` _minz _returnvalue_2))
  (set `self.C` (`KismetMathLibrary.MakeVector` _maxz _returnvalue))
  (set `self.D` (`KismetMathLibrary.MakeVector` _maxz _returnvalue_2))
  (set `/Game/ui/kinectHUD.viewing frustum` (make `/Game/DataStructure/ViewingFrustum` _returnvalue_2 _returnvalue_2 _minz _maxz) (`self.kinect HUD`)))

(fn `ResumeTo`
  (params (`player state` :type "/Game/DataStructure/PLAYER_STATE Enum" :default "NewEnumerator0"))
  (bind _player_character (`self.player character`))
  (bind _returnvalue (`|EnumEquality` (`self.pause player state`) "NewEnumerator2"))
  (if (`|EnumEquality` `player state` "NewEnumerator2")
    (if _returnvalue
      (`RedCharacter.ResumeJump` _player_character)
      (else
        (`RedCharacter.ReadyJump` _player_character)))
    (elif _returnvalue
      (`RedCharacter.cancelJump` _player_character)))
  (set `self.player state` `player state`))

(fn `UserConstructionScript`)