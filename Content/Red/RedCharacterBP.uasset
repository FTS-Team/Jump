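; RedCharacterBP is the player character Blueprint for a jumping game, handling UI and sound feedback.
; BeginPlay shows the HUD, P opens a reusable pause menu, and GameOverDrive shows the End screen, with both screens pausing the game.
; Drive events, with no callers in this graph, switch charge-up intro and loop sounds for jump power and play the score sound.
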(event `self.ReceiveBeginPlay`
  ;[1 1 1] create HUDReference and show HUD widget
  (`GameplayStatics.PlaySound2D` "/Game/Audio/S_start.S_start")
  (bind _returnvalue (`|CreateWidget` "/Game/ui/HUD.HUD_C"))
  (bind _output_get (set `self.HUDReference` _returnvalue))
  (`UserWidget.AddToViewport` _output_get 0)
  (`WidgetBlueprintLibrary.SetInputMode_GameOnly` (`GameplayStatics.GetPlayerController` 0)))

(event `Key|P`
  (params (Key :type "Key Structure"))
  (bind _returnvalue (`GameplayStatics.GetPlayerController` 0))
  (bind _pausemenureference (`self.PauseMenuReference`))
  ;[1 1 1] keyboard P  PauseMenu
  (:`Pressed`
    (`/Engine/EditorBlueprintResources/StandardMacros.IsValid` _pausemenureference
      (:`Is Valid`
        _)
      (:`Is Not Valid`
        (bind _returnvalue_2 (`|CreateWidget` "/Game/ui/PauseMenu.PauseMenu_C"))
        (set `self.PauseMenuReference` _returnvalue_2)))
    (`WidgetBlueprintLibrary.SetInputMode_UIOnlyEx` _returnvalue _pausemenureference)
    (`UserWidget.AddToViewport` _pausemenureference 0)
    (`GameplayStatics.SetGamePaused` true)
    (set `PlayerController.bShowMouseCursor` true _returnvalue)))

(event `self.GameOverDrive`
  (bind _returnvalue (`GameplayStatics.GetPlayerController` 0))
  ;[1 1 1] GameOver End
  (`GameplayStatics.PlaySound2D` "/Game/Audio/S_fall.S_fall")
  (bind _returnvalue_2 (`|CreateWidget` "/Game/ui/End.End_C"))
  (`UserWidget.AddToViewport` _returnvalue_2 0)
  (`WidgetBlueprintLibrary.SetInputMode_GameAndUIEx` _returnvalue)
  (`GameplayStatics.SetGamePaused` true)
  (set `PlayerController.bShowMouseCursor` true _returnvalue))

(event `self.ReadyJumpDrive`
  ;[1 1 1] setPowerSound
  (`AudioComponent.Play` (`self.Sound_PowerIntro`) 0.0))

(event `self.FullPowerDrive`
  ;[1 1 1] setPowerSound
  (`AudioComponent.Stop` (`self.Sound_PowerIntro`))
  (`AudioComponent.Play` (`self.Sound_PowerLoop`) 0.0))

(event `self.StartJumpDrive`
  ;[1 1 1] setPowerSound
  (`AudioComponent.Stop` (`self.Sound_PowerIntro`))
  (`AudioComponent.Stop` (`self.Sound_PowerLoop`)))

(event `self.AddScoreDrive`
  ;[1 1 1] setAddScoreSound
  (`GameplayStatics.PlaySound2D` "/Game/Audio/S_success.S_success"))

(fn `UserConstructionScript`)